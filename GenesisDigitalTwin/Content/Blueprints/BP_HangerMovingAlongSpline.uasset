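; BP_HangerMovingAlongSpline spawns a hanger vehicle at each spline point and advances them around the spline like a stepped conveyor between processes.
; MoveToNextProcess plays a Timeline that interpolates each hanger to its next point, wrapping through the spline's end.
; On finish, it increments indices, reveals process meshes and calls CallAllHangerArrived.
; A Gate closes after StartMoveCall until EnableMoveCall reopens it; older continuous-loop movement remains unused.
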(event Custom|MoveToNextLocation
  (bind _currenttargetpoint (Variables|Default|GetCurrentTargetPoint))
  (bind _spline (Variables|Default|GetSpline))
  (bind _returnvalue (Spline|GetDistanceAlongSplineatSplinePoint _spline _currenttargetpoint))
  (bind _returnvalue_2 (- _currenttargetpoint 1))
  (bind _returnvalue_3 (Spline|GetDistanceAlongSplineatSplinePoint _spline _returnvalue_2))
  (bind _returnvalue_4 (Math|Float|Lerp _returnvalue_3 _returnvalue 0.0))
  (for _array_element (Variables|Default|GetHangers)
    (Transformation|SetActorLocationAndRotation _array_element (Spline|GetLocationatDistanceAlongSpline _spline _returnvalue_4 "World") (Spline|GetRotationatDistanceAlongSpline (Variables|Default|GetSpline) _returnvalue_4 "World"))))

(event Custom|StartMoveCall
  (Utilities|FlowControl|Sequence ; 실행 핀을 여러 갈래로 순서대로 실행시키는 노드
    (:then_0
      (Utilities|FlowControl|Gate false :!label _label))
    (:then_1
      (goto _label Close))))

(event Custom|EnableMoveCall
  (Utilities|FlowControl|Gate false) ; enters at Open
)

(event Custom|MoveToNextProcess
  (bind _hangers (Variables|Default|GetHangers))
  (bind _spline (Variables|Default|GetSpline))
  (Development|PrintString "MoveToNextProcess Called")
  (bind _newtrack_0 (Timeline|Timeline_0 PlayFromStart) ; play from start : 처음부터 시작
    (:Update
      (for _array_element _hangers ; 배열에 들어있는 모든 요소를 하나씩 꺼내서 반복 실행하는 노드
        (Transformation|SetActorTransform _array_element (Spline|GetTransformatDistanceAlongSpline _spline (Math|Float|Lerp (Spline|GetDistanceAlongSplineatSplinePoint _spline (Variables|/Game/Blueprints/BP_HangerVehicle.BP_HangerVehicle_C|GetCurrentPointIndex _array_element)) (Math|Float|SelectFloat (Spline|GetSplineLength _spline) (Spline|GetDistanceAlongSplineatSplinePoint _spline (Math|Integer|%(Integer) (+ (Variables|/Game/Blueprints/BP_HangerVehicle.BP_HangerVehicle_C|GetCurrentPointIndex _array_element) 1) (Spline|GetNumberOfSplinePoints _spline))) (== (Math|Integer|%(Integer) (+ (Variables|/Game/Blueprints/BP_HangerVehicle.BP_HangerVehicle_C|GetCurrentPointIndex _array_element) 1) (Spline|GetNumberOfSplinePoints _spline)) 0)) _newtrack_0) "World" false))))
    (:Finished
      (for _array_element_2 _hangers
        (bind _output_get (Variables|/Game/Blueprints/BP_HangerVehicle.BP_HangerVehicle_C|SetCurrentPointIndex _array_element_2 (Math|Integer|%(Integer) (+ (Variables|/Game/Blueprints/BP_HangerVehicle.BP_HangerVehicle_C|GetCurrentPointIndex _array_element_2) 1) (Spline|GetNumberOfSplinePoints (Variables|Default|GetSpline)))))
        (Default|RevealProcessMesh _array_element_2 _output_get))
      (Default|CallAllHangerArrived))))

(event EventBeginPlay
  (bind _spline (Variables|Default|GetSpline))
  (bind _returnvalue (Actor|GetActorOfClass "/Game/Blueprints/BP_ProcessManager.BP_ProcessManager_C"))
  (Variables|Default|SetProcessManagerRef _returnvalue)
  (Utilities|Array|Clear (Variables|Default|GetHangers))
  (for _index (range 0 (- (Spline|GetNumberOfSplinePoints _spline) 1))
    (bind _returnvalue_2 (Game|SpawnActorfromClass "/Game/Blueprints/BP_HangerVehicle.BP_HangerVehicle_C" (Spline|GetTransformatSplinePoint _spline _index "World" false) "Undefined" "MultiplyWithRoot" 0 _index 0))
    (Variables|/Game/Blueprints/BP_HangerVehicle.BP_HangerVehicle_C|SetCurrentPointIndex _returnvalue_2 _index)
    (Utilities|Array|AddUnique (Variables|Default|GetHangers) _returnvalue_2)))

(fn ConstructionScript
  (bind _spline (Variables|Default|GetSpline))
  (for (_array_element _array_index) (Variables|Default|GetHangers) ; F + 좌클릭
    (Transformation|SetActorLocationAndRotation _array_element (Spline|GetLocationatDistanceAlongSpline _spline (* _array_index (Variables|Default|GetDistanceBetweenTheActors)) "World") (Spline|GetRotationatDistanceAlongSpline _spline (Variables|Default|GetMovingSplineDistance) "World"))))

(fn NotifyRobotFinished)