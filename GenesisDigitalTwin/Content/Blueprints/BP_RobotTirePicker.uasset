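; Robot arm actor that picks a target tire and places it at a destination point, using a baked conveyor-to-table animation.
; StartPickAndPlace checks busy and pickable state, then uses timed delays to attach the tire to the grip socket, detach and snap it, then flag it mountable.
; BeginPlay maps the mesh to Control Rig and aligns an IK target, but the IK and timeline-driven movement logic is disconnected.
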(event Custom|StartPickAndPlace
  (if (not (Variables|Default|GetIsBusy))
    (Utilities|IsValid (Variables|Default|GetTargetTire)
      (:Is%20Valid
        (if (Variables|/Game/Blueprints/BP_Tire.BP_Tire_C|GetCanBePicked (Variables|Default|GetTargetTire))
          (Variables|Default|SetIsBusy true)
          (Variables|/Game/Blueprints/BP_Tire.BP_Tire_C|SetCanBePicked (Variables|Default|GetTargetTire) false)
          (Components|Animation|PlayAnimation (Variables|Default|GetRobotMesh) "/Game/Meshes/Robot/Anim_Robot_ConveyorToTable_Base.Anim_Robot_ConveyorToTable_Base" false)
          (Utilities|FlowControl|Delay (Variables|Default|GetAttachTime))
          (Transformation|AttachComponentToComponent (Variables|Default|GetTargetTire) (Variables|Default|GetRobotMesh) "TireGripSocket" "SnapToTarget" "SnapToTarget" "KeepWorld" true)
          (Utilities|FlowControl|Delay (- (Variables|Default|GetDetachTime) (Variables|Default|GetAttachTime)))
          (Transformation|DetachFromActor (Variables|Default|GetTargetTire) "KeepWorld" "KeepWorld" "KeepWorld")
          (Transformation|SetActorLocation (Variables|Default|GetTargetTire) (Transformation|GetWorldLocation (Variables|Default|GetDestPointRef)) false false)
          (Utilities|FlowControl|Delay (- (Variables|Default|GetAnimEndTime) (Variables|Default|GetDetachTime)))
          (Variables|Default|SetIsBusy false)
          (Variables|/Game/Blueprints/BP_Tire.BP_Tire_C|SetCanBeMounted (Variables|Default|GetTargetTire) true)
          (Variables|/Game/Blueprints/BP_Tire.BP_Tire_C|SetCanBePicked (Variables|Default|GetTargetTire) false))))))

(event EventTick
  (params (DeltaSeconds :type Float%20%28single-precision%29)))

(event EventBeginPlay
  (Class|ControlRigComponent|AddMappedCompleteSkeletalMesh (Variables|Default|GetCR_Component) (Variables|Default|GetRobotMesh) "Output")
  (Transformation|SetWorldTransform (Variables|Default|GetIK_Target) (Transformation|GetSocketTransform (Variables|Default|GetRobotMesh) "TireGripSocket" "RTS_World") false false))

(fn ConstructionScript)