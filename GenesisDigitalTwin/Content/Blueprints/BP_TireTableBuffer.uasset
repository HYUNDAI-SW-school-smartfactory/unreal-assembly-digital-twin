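; BP_TireTableBuffer is a table that buffers tires between a conveyor and their removal for mounting.
; AddTireToTable detaches an incoming tire, snaps it to the next of five stack points, marks it mountable but not pickable, and stops the conveyor at capacity.
; TakeTireFromTable pops the most recently added tire, then RequestNextTire tells the referenced conveyor to spawn a replacement while space remains.
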(event EventBeginPlay
  (Utilities|Array|Clear (Variables|Default|GetStoredTires))
  (Variables|Default|SetStackPoints (Utilities|Array|MakeArray (Variables|Default|GetPoint1) (Variables|Default|GetPoint2) (Variables|Default|GetPoint3) (Variables|Default|GetPoint4) (Variables|Default|GetPoint5))))

(fn ConstructionScript)

(fn AddTiretoTable
  (params (IncomingTire :type BP%20Tire%20Object%20Reference))
  (bind _stackpoints (Variables|Default|GetStackPoints))
  (bind _storedtires (Variables|Default|GetStoredTires))
  (bind _returnvalue (Utilities|Array|Length _storedtires))
  (bind _output (Utilities|Array|Get(acopy) _stackpoints _returnvalue))
  (Development|PrintString (Utilities|String|Append "Buffer Count: " (Utilities|String|ToString(Integer) (Utilities|Array|Length (Variables|Default|GetStoredTires)))))
  (if (< (Utilities|Array|Length (Variables|Default|GetStoredTires)) (Variables|Default|GetMaxCapacity))
    (Utilities|IsValid IncomingTire
      (:Is%20Valid
        (Transformation|DetachFromActor IncomingTire "KeepWorld" "KeepWorld" "KeepWorld")
        (Transformation|SetActorTransform IncomingTire (Math|Transform|MakeTransform (Transformation|GetWorldLocation _output) (Transformation|GetWorldRotation _output)) false true)
        (Rendering|SetActorHiddenInGame IncomingTire false)
        (Variables|/Game/Blueprints/BP_Tire.BP_Tire_C|SetCanBePicked IncomingTire false)
        (Variables|/Game/Blueprints/BP_Tire.BP_Tire_C|SetCanBeMounted IncomingTire true)
        (Utilities|Array|AddUnique (Variables|Default|GetStoredTires) IncomingTire)
        (if (>= (Utilities|Array|Length (Variables|Default|GetStoredTires)) (Variables|Default|GetMaxCapacity))
          (Utilities|IsValid (Variables|Default|GetConveyorRef)
            (:Is%20Valid
              (Default|StopConveyor (Variables|Default|GetConveyorRef))
              (return true))
            (:Is%20Not%20Valid
              (return true)))
          (else
            (return true))))
      (:Is%20Not%20Valid
        (return false)))
    (else
      (return false))))

(fn TakeTirefromTable
  (if (> (Utilities|Array|Length (Variables|Default|GetStoredTires)) 0)
    (LocalVariables|SetSelectedTire (Utilities|Array|Get(acopy) (Variables|Default|GetStoredTires) (Utilities|Array|LastIndex (Variables|Default|GetStoredTires))))
    (Utilities|Array|RemoveIndex (Variables|Default|GetStoredTires) (Utilities|Array|LastIndex (Variables|Default|GetStoredTires)))
    (CallFunction|RequestNextTire)
    (return (LocalVariables|GetSelectedTire) true)
    (else
      (return 0 false))))

(fn GetStoredCount
  (return (Utilities|Array|Length (Variables|Default|GetStoredTires))))

(fn RequestNextTire
  (if (< (Utilities|Array|Length (Variables|Default|GetStoredTires)) (Variables|Default|GetMaxCapacity))
    (Utilities|IsValid (Variables|Default|GetConveyorRef)
      (:Is%20Valid
        (Default|SpawnNextTire (Variables|Default|GetConveyorRef))))
    (else
      (Utilities|IsValid (Variables|Default|GetConveyorRef)
        (:Is%20Valid
          (Default|StopConveyor (Variables|Default|GetConveyorRef)))))))