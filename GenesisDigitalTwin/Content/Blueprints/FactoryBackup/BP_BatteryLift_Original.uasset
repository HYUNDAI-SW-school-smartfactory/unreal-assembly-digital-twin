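; Factory battery lift Blueprint that animates a battery pack being raised for installation when StartBatteryInstall is called.
; BeginPlay caches the lift root's start position and derives the raised position from LiftHeight.
; A timeline lerps the root upward, waits briefly, hides the pack as if installed, then reverses to lower the lift.
; An IsInstalling flag blocks re-triggering until the lift returns.
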(event Custom|StartBatteryInstall
  (if (not (Variables|Default|GetIsInstalling))
    (Variables|Default|SetIsInstalling true)
    (Rendering|SetVisibility (Variables|Default|GetBatteryPack) true false)
    (bind (_direction _liftalpha) (Timeline|TL_Lift PlayFromStart)
      (:Update
        (Transformation|SetRelativeLocation (Variables|Default|GetLiftRoot) (Math|Vector|Lerp(Vector) (Variables|Default|GetLiftStartLocation) (Variables|Default|GetLiftEndLocation) _liftalpha) false false))
      (:Finished
        (if (Utilities|Enum|Equal(Enum) _direction "Forward")
          (Utilities|FlowControl|Delay 2.0)
          (Rendering|SetVisibility (Variables|Default|GetBatteryPack) false false)
          (Timeline|TL_Lift Reverse)
          (else
            (Variables|Default|SetIsInstalling false)))))))

(event EventBeginPlay
  (bind _output_get (Variables|Default|SetLiftStartLocation (Variables|/Script/Engine.SceneComponent|GetRelativeLocation (Variables|Default|GetLiftRoot))))
  (Variables|Default|SetLiftEndLocation (+ _output_get (Math|Vector|MakeVector 0.0 0.0 (Variables|Default|GetLiftHeight)))))

(fn ConstructionScript)