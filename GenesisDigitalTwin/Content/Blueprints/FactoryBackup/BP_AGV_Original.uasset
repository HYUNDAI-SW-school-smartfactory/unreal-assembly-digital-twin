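; An automated guided vehicle (AGV) actor that shuttles a battery pack along a waypoint path in a factory scene.
; While moving, Tick turns it toward the current waypoint and steps it there at constant speed, advancing within an acceptance radius.
; At the last waypoint it hides the pack, starts installation on the battery lift and reverses.
; Back at the first waypoint, it shows the pack and heads out again.
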(event EventTick
  (params (DeltaSeconds :type Float%20%28single-precision%29))
  (bind _returnvalue (Transformation|GetActorLocation))
  (if (Variables|Default|GetblsMoving)
    (Transformation|SetActorRotation (Math|Rotator|FindLookatRotation _returnvalue (Utilities|Array|Get(acopy) (Variables|Default|GetWaypoints) (Variables|Default|GetCurrentWaypointIndex))))
    (Transformation|SetActorLocation (Math|Interpolation|VInterptoConstant _returnvalue (Utilities|Array|Get(acopy) (Variables|Default|GetWaypoints) (Variables|Default|GetCurrentWaypointIndex)) DeltaSeconds (Variables|Default|GetMoveSpeed)) false false)
    (if (<= (Math|Vector|Distance(Vector) (Math|Interpolation|VInterptoConstant _returnvalue (Utilities|Array|Get(acopy) (Variables|Default|GetWaypoints) (Variables|Default|GetCurrentWaypointIndex)) DeltaSeconds (Variables|Default|GetMoveSpeed)) (Utilities|Array|Get(acopy) (Variables|Default|GetWaypoints) (Variables|Default|GetCurrentWaypointIndex))) (Variables|Default|GetAcceptanceRadius))
      (if (Variables|Default|GetGoingForward)
        (if (< (+ (Variables|Default|GetCurrentWaypointIndex) 1) (Utilities|Array|Length (Variables|Default|GetWaypoints)))
          (Rendering|SetVisibility (Variables|Default|GetBatteryPack_Mesh) true true)
          (Variables|Default|SetCurrentWaypointIndex (+ (Variables|Default|GetCurrentWaypointIndex) 1))
          (else
            (Rendering|SetVisibility (Variables|Default|GetBatteryPack_Mesh) false true)
            (Default|StartBatteryInstall (Variables|Default|GetBatteryLiftRef))
            (Variables|Default|SetGoingForward false)
            (Variables|Default|SetCurrentWaypointIndex (- (Variables|Default|GetCurrentWaypointIndex) 1))))
        (elif (>= (- (Variables|Default|GetCurrentWaypointIndex) 1) 0)
          (Variables|Default|SetCurrentWaypointIndex (- (Variables|Default|GetCurrentWaypointIndex) 1))
          (else
            (Rendering|SetVisibility (Variables|Default|GetBatteryPack_Mesh) true true)
            (Variables|Default|SetGoingForward true)
            (Variables|Default|SetCurrentWaypointIndex (+ (Variables|Default|GetCurrentWaypointIndex) 1))))))))

(event EventBeginPlay)

(fn ConstructionScript)