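; BP_TireAssemblyCell_Original is a factory cell that moves tires from a conveyor to a table buffer, then to a car.
; BeginPlay casts its conveyor, buffer and two robot child actors, wires their references and pick/drop points, then spawns the first tire.
; Tick polls both stages: the first robot picks pickable conveyor tires when idle.
; The second starts mounting when idle and the buffer holds at least two.
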(event EventBeginPlay
  (bind _asbp_tire_table_buffer (Utilities|Casting|CastToBP_TireTableBuffer (Variables|/Script/Engine.ChildActorComponent|GetChildActor (Variables|Default|GetTireTableBuffer))))
  (Variables|Default|SetTireTableBufferRef _asbp_tire_table_buffer)
  (bind _asbp_tire_conveyor (Utilities|Casting|CastToBP_TireConveyor (Variables|/Script/Engine.ChildActorComponent|GetChildActor (Variables|Default|GetConveyorActor))))
  (Variables|Default|SetConveyorRef _asbp_tire_conveyor)
  (bind _asbp_robot_tire_picker (Utilities|Casting|CastToBP_RobotTirePicker (Variables|/Script/Engine.ChildActorComponent|GetChildActor (Variables|Default|GetRobot_ConveyorToTable))))
  (Variables|Default|SetRobotToTableRef _asbp_robot_tire_picker)
  (bind _asbp_robot_tire_picker_to_car (Utilities|Casting|CastToBP_RobotTirePickerToCar (Variables|/Script/Engine.ChildActorComponent|GetChildActor (Variables|Default|GetRobot_TableToCar))))
  (Variables|Default|SetRobotToCarRef _asbp_robot_tire_picker_to_car)
  (Variables|/Game/Blueprints/BP_TireTableBuffer.BP_TireTableBuffer_C|SetConveyorRef (Variables|Default|GetTireTableBufferRef) (Variables|Default|GetConveyorRef))
  (Variables|/Game/Blueprints/BP_RobotTirePicker.BP_RobotTirePicker_C|SetTableBufferRef (Variables|Default|GetRobotToTableRef) (Variables|Default|GetTireTableBufferRef))
  (Variables|/Game/Blueprints/BP_RobotTirePicker.BP_RobotTirePicker_C|SetConveyorRef (Variables|Default|GetRobotToTableRef) (Variables|Default|GetConveyorRef))
  (Variables|/Game/Blueprints/BP_RobotTirePicker.BP_RobotTirePicker_C|SetSourcePointRef (Variables|Default|GetRobotToTableRef) (Variables|Default|GetP_ConveyorPickup))
  (Variables|/Game/Blueprints/BP_RobotTirePicker.BP_RobotTirePicker_C|SetDestPointRef (Variables|Default|GetRobotToTableRef) (Variables|Default|GetP_TableDrop))
  (Variables|/Game/Blueprints/BP_RobotTirePickerToCar.BP_RobotTirePickerToCar_C|SetTableBufferRef (Variables|Default|GetRobotToCarRef) (Variables|Default|GetTireTableBufferRef))
  (Variables|/Game/Blueprints/BP_RobotTirePickerToCar.BP_RobotTirePickerToCar_C|SetSourcePointRef (Variables|Default|GetRobotToCarRef) (Variables|Default|GetP_TablePickup))
  (Variables|/Game/Blueprints/BP_RobotTirePickerToCar.BP_RobotTirePickerToCar_C|SetDestPointRef (Variables|Default|GetRobotToCarRef) (Variables|Default|GetP_CarMount))
  (Default|SpawnNextTire (Variables|Default|GetConveyorRef)))

(event EventTick
  (params (DeltaSeconds :type Float%20%28single-precision%29))
  (Utilities|IsValid (Variables|Default|GetTireTableBufferRef)
    (:Is%20Valid
      (Utilities|FlowControl|Sequence
        (:then_0
          (Utilities|IsValid (Variables|/Game/Blueprints/BP_TireConveyor.BP_TireConveyor_C|GetTargetTire (Variables|Default|GetConveyorRef))
            (:Is%20Valid
              (if (and (Variables|/Game/Blueprints/BP_Tire.BP_Tire_C|GetCanBePicked (Variables|/Game/Blueprints/BP_TireConveyor.BP_TireConveyor_C|GetTargetTire (Variables|Default|GetConveyorRef))) (not (Variables|/Game/Blueprints/BP_RobotTirePicker.BP_RobotTirePicker_C|GetIsBusy (Variables|Default|GetRobotToTableRef))))
                (Variables|/Game/Blueprints/BP_RobotTirePicker.BP_RobotTirePicker_C|SetTargetTire (Variables|Default|GetRobotToTableRef) (Variables|/Game/Blueprints/BP_TireConveyor.BP_TireConveyor_C|GetTargetTire (Variables|Default|GetConveyorRef)))
                (Default|StartPickandPlace (Variables|Default|GetRobotToTableRef))))))
        (:then_1
          (bind _count (Default|GetStoredCount (Variables|Default|GetTireTableBufferRef)))
          (if (and (>= _count 2) (not (Variables|/Game/Blueprints/BP_RobotTirePickerToCar.BP_RobotTirePickerToCar_C|GetIsBusy (Variables|Default|GetRobotToCarRef))))
            (Default|StartMountTire (Variables|Default|GetRobotToCarRef))))))))

(fn ConstructionScript)