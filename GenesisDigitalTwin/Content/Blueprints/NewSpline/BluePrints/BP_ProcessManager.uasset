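; BP_ProcessManager is a coordinator actor that links hangers on lanes to process robots.
; On BeginPlay it registers itself with every BP_Hanger and caches all BP_Robot actors; lanes are added uniquely through RegisterLane.
; HangerArrived prints the lane point's process type, then rebuilds SelectedRobots with robots matching CurrentProcessType, a variable not assigned in this graph.
; The selected robots receive no commands here.
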(event Custom|HangerArrived
  (params (Hanger :type BP%20Hanger%20Object%20Reference) (PointID :type Integer))
  (Development|PrintString (Utilities|String|EnumtoString (.ProcessType (Utilities|Struct|BreakST_PointData (Default|GetPoint (Variables|/Game/Blueprints/NewSpline/BluePrints/BP_Hanger.BP_Hanger_C|GetLaneReference Hanger) (Variables|/Game/Blueprints/NewSpline/BluePrints/BP_Hanger.BP_Hanger_C|GetCurrentPointID Hanger))))))
  (Utilities|Array|Clear (Variables|Default|GetSelectedRobots))
  (for _array_element (Variables|Default|GetAllRobots)
    (if (Utilities|Enum|Equal(Enum) (Variables|/Game/Blueprints/NewSpline/BluePrints/BP_Robot.BP_Robot_C|GetProcessType _array_element) (Variables|Default|GetCurrentProcessType))
      (Utilities|Array|Add (Variables|Default|GetSelectedRobots) _array_element))))

(event EventBeginPlay
  (bind _outactors (Actor|GetAllActorsOfClass "/Game/Blueprints/NewSpline/BluePrints/BP_Hanger.BP_Hanger_C"))
  (for _array_element _outactors
    (Default|RegisterProcessManager _array_element self))
  (Development|PrintString "All Hangers Registered")
  (bind _outactors_2 (Actor|GetAllActorsOfClass "/Game/Blueprints/NewSpline/BluePrints/BP_Robot.BP_Robot_C"))
  (Variables|Default|SetAllRobots _outactors_2)
  (Development|PrintString "All Robots Registered"))

(fn ConstructionScript)

(fn RegisterLane
  (params (Lane :type BP%20Lane%20Object%20Reference))
  (Utilities|Array|AddUnique (Variables|Default|GetRegisteredLanes) Lane)
  (Development|PrintString "Lane Registered") ; 디버깅용
)