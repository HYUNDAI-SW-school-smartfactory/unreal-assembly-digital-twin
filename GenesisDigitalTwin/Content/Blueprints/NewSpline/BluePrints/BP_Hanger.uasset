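; BP_Hanger is a hanger actor that travels point to point along a lane spline.
; On BeginPlay it snaps to its current point, then tries to reserve the next one on LaneReference, setting a short retry timer if refused.
; A timeline interpolates spline distance to drive its transform.
; On arrival it releases the previous point and notifies the registered process manager.
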(event Custom|MoveToPoint
  (params (Target%20Point :type Integer))
  (CallFunction|CalculateMove Target%20Point)
  (bind _success (Default|TryReservePoint (Variables|Movement|GetLaneReference) Target%20Point (Variables|Identity|GetHangerID)))
  (if _success
    (CallFunction|StartMove)
    (else
      (Utilities|Time|SetTimerbyEvent (EventDispatchers|CreateEvent :!event Custom|RetryMove) 0.2))))

(event Custom|StartMove
  (Variables|Default|SetStartDistance (Variables|Movement|GetCurrentDistance))
  (bind __alpha (Timeline|TL_Move PlayFromStart)
    (:Update
      (bind _output_get (Variables|Movement|SetCurrentDistance (Math|Float|Lerp (Variables|Default|GetStartDistance) (Variables|Movement|GetTargetDistance) __alpha)))
      (Transformation|SetActorTransform (Spline|GetTransformatDistanceAlongSpline (Variables|/Game/Blueprints/NewSpline/BluePrints/BP_Lane.BP_Lane_C|GetLaneSpline (Variables|Movement|GetLaneReference)) _output_get "World" false)))
    (:Finished
      (Default|ReleasePoint (Variables|Movement|GetLaneReference) (Variables|Movement|GetCurrentPointID))
      (Variables|Movement|SetCurrentPointID (Variables|Movement|GetTargetPointID))
      (Default|HangerArrived (Variables|Default|GetProcessManagerReference) self (Variables|Movement|GetCurrentPointID)))))

(event Custom|RetryMove
  (CallFunction|MovetoPoint (Variables|Movement|GetTargetPointID)))

(event EventBeginPlay
  (CallFunction|Initialize)
  (CallFunction|MovetoPoint (+ (Variables|Movement|GetCurrentPointID) 1)))

(fn ConstructionScript)

(fn Initialize
  (Utilities|IsValid (Variables|Movement|GetLaneReference)
    (:Is%20Valid
      (CallFunction|InitializeonLane))
    (:Is%20Not%20Valid
      (Development|PrintString "LaneReference is NULL" true true "(R=1.000000,G=0.000000,B=0.000000,A=1.000000)" 5.0))))

(fn InitializeonLane
  (bind _lanereference (Variables|Movement|GetLaneReference))
  (bind _output_get (Variables|Movement|SetCurrentDistance (Default|GetPointDistance _lanereference (Variables|Movement|GetCurrentPointID))))
  (Transformation|SetActorTransform (Default|GetTransformatDistance _lanereference _output_get) false true))

(fn CalculateMove
  (params (TargetPoint :type Integer))
  (Variables|Movement|SetTargetDistance (* TargetPoint (Variables|/Game/Blueprints/NewSpline/BluePrints/BP_Lane.BP_Lane_C|GetPointSpacing (Variables|Movement|GetLaneReference))))
  (Variables|Default|SetStartDistance (* (Variables|Movement|GetCurrentPointID) (Variables|/Game/Blueprints/NewSpline/BluePrints/BP_Lane.BP_Lane_C|GetPointSpacing (Variables|Movement|GetLaneReference)))))

(fn RegisterProcessManager
  (params (NewProcessManager :type BP%20Process%20Manager%20Object%20Reference))
  (Variables|Default|SetProcessManagerReference NewProcessManager)
  (Development|PrintString "ProcessManager Registered"))