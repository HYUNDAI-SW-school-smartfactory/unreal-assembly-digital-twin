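; BP_Lane is a spline lane that provides numbered stop points hangers can reserve and release.
; On BeginPlay it optionally samples LaneSpline at PointSpacing into point structs with transform, distance and occupier, then registers with BP_ProcessManager.
; Reservation succeeds only on free points (occupier -1); SetPointOccupier is left unwired and ignores its new occupier.
; It also serves point lookups and clamped transform-at-distance queries, and draws persistent debug spheres and IDs after generation.
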(event EventBeginPlay
  (Utilities|FlowControl|Sequence
    (:then_0
      (if (Variables|Default|GetGenerateOnBeginPlay) ; 자동생성 On/Off
        (CallFunction|GeneratePoints)))
    (:then_1
      (bind _returnvalue (Actor|GetActorOfClass "/Game/Blueprints/NewSpline/BluePrints/BP_ProcessManager.BP_ProcessManager_C"))
      (Default|RegisterLane _returnvalue self))))

(fn ConstructionScript)

(fn GeneratePoints
  (Utilities|Array|Clear (Variables|Default|GetPoints))
  (for _index (range 0 (Math|Float|Floor (/ (Spline|GetSplineLength (Variables|Default|GetLaneSpline)) (Variables|Default|GetPointSpacing))))
    (Utilities|Array|Add (Variables|Default|GetPoints) (Utilities|Struct|MakeST_PointData _index (Spline|GetLocationatDistanceAlongSpline (Variables|Default|GetLaneSpline) (* _index (Variables|Default|GetPointSpacing)) "World") (Spline|GetRotationatDistanceAlongSpline (Variables|Default|GetLaneSpline) (* _index (Variables|Default|GetPointSpacing)) "World") (* _index (Variables|Default|GetPointSpacing)) "NewEnumerator0" -1 "NewEnumerator0" (Variables|Default|GetLaneID))))
  (CallFunction|DrawDebugPoints))

(fn DrawDebugPoints
  (for _array_element (Variables|Default|GetPoints)
    (Rendering|Debug|DrawDebugSphere (.Location (Utilities|Struct|BreakST_PointData _array_element)) 2e+01 12 "(R=1.000000,G=1.000000,B=1.000000,A=1.000000)" 999999.0 2.0)
    (Rendering|Debug|DrawDebugString (.Location (Utilities|Struct|BreakST_PointData _array_element)) (Utilities|String|ToString(Integer) (.PointID (Utilities|Struct|BreakST_PointData _array_element))) 0 "(R=1.000000,G=1.000000,B=1.000000,A=1.000000)" 999999.0)))

(fn GetPoint
  (params (PointID :type Integer))
  (bind _points (Variables|Default|GetPoints))
  (if (Utilities|Array|IsValidIndex _points PointID)
    (return (Utilities|Array|Get(acopy) _points PointID))
    (else
      (Development|PrintString "Invalid PointID" true true "(R=1.000000,G=0.000000,B=0.000000,A=1.000000)" 5.0))))

(fn GetPointDistance
  (params (PointID :type Integer))
  (return (.Distance (Utilities|Struct|BreakST_PointData (PointAPI|GetPoint PointID)))))

(fn GetPointLocation
  (params (PointID :type Integer))
  (return (.Location (Utilities|Struct|BreakST_PointData (PointAPI|GetPoint PointID)))))

(fn IsValidPoint
  (params (PointID :type Integer))
  (return (Utilities|Array|IsValidIndex (Variables|Default|GetPoints) PointID)))

(fn GetTransformatDistance
  (params (Distance :type Float%20%28double-precision%29))
  (bind _lanespline (Variables|Default|GetLaneSpline))
  (return (Spline|GetTransformatDistanceAlongSpline _lanespline (Math|Float|Clamp(Float) Distance 0.0 (Spline|GetSplineLength _lanespline)) "World" false)))

(fn TryReservePoint
  (params (PointID :type Integer) (HangerID :type Integer))
  (bind _pointdata (PointAPI|GetPoint PointID))
  (if (== (.OccupyingHanger (Utilities|Struct|BreakST_PointData _pointdata)) -1)
    (bind _structout (Utilities|Struct|SetmembersinST_PointData _pointdata HangerID))
    (Utilities|Array|SetArrayElem (Variables|Default|GetPoints) PointID _structout)
    (return true)
    (else
      (return false))))

(fn SetPointOccupier
  (params (PointID :type Integer) (NewOccupier :type BP%20Hanger%20Object%20Reference))
  (Utilities|Array|SetArrayElem :TargetArray (Variables|Default|GetPoints) :Index PointID))

(fn ReleasePoint
  (params (PointID :type Integer))
  (bind _structout (Utilities|Struct|SetmembersinST_PointData (PointAPI|GetPoint PointID) -1))
  (Utilities|Array|SetArrayElem (Variables|Default|GetPoints) PointID _structout))