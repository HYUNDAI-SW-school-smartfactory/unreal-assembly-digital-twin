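; BP_ProcessManager coordinates a production-line cycle between robots and hangers moving along a spline.
; On BeginPlay it binds to every BP_RobotBase's finished event, records the robot count, and binds to the hanger actor's all-arrived event.
; When all robots report finished, it tells the hanger to move to the next process.
; On arrival it resets the count and calls StartAllProcess, with leftover test print and delay.
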(event Custom|Robot%20FinishedReceived
  (params (ProcessIndex :type Integer))
  (bind _output_get (Variables|Default|SetFinishedRobotCount (+ (Variables|Default|GetFinishedRobotCount) 1)))
  (if (>= _output_get (Variables|Default|GetTotalRobotCount))
    (Development|PrintString "All Robot Finished")
    (Default|MovetoNextProcess (Variables|Default|GetHangerRef))))

(event Custom|HangersArrivedReceived
  (Variables|Default|SetFinishedRobotCount 0)
  (Default|CallStartAllProcess)
  ;[0.15 0.15 0.15 0.5] 로봇 작업 부, 각 로봇이 완료되면 Finished Robot Count를 늘려야함
  (Development|PrintString "Run Process") ; 테스트용
  (Utilities|FlowControl|Delay 1e+01) ; 테스트용
)

(event EventBeginPlay
  (Utilities|FlowControl|Sequence
    (:then_0
      (bind _outactors (Actor|GetAllActorsOfClass "/Game/Blueprints/BP_RobotBase.BP_RobotBase_C"))
      (for _array_element _outactors
        (EventDispatchers|BindEventtoRobotFinished _array_element (delegate Custom|Robot%20FinishedReceived)))
      (Variables|Default|SetTotalRobotCount (Utilities|Array|Length _outactors)))
    (:then_1
      (bind _returnvalue (Actor|GetActorOfClass "/Game/Blueprints/BP_HangerMovingAlongSpline.BP_HangerMovingAlongSpline_C"))
      (bind _output_get (Variables|Default|SetHangerRef _returnvalue))
      (EventDispatchers|BindEventtoAllHangerArrived _output_get (delegate Custom|HangersArrivedReceived)))))

(fn ConstructionScript)