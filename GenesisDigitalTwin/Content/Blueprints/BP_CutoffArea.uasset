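; BP_CutoffArea is a placeable actor that publishes an axis-aligned box region to the MPC_CutoffArea material parameter collection.
; CutoffIndex selects one of four Min/Max point parameter pairs for the actor to write.
; The corners come from actor location plus or minus scale times 50, matching a 100-unit cube and ignoring rotation.
; The construction script and BeginPlay both push the values, covering editor changes and game start but not runtime movement.
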(event Custom|SetMaterialParameter
  (bind _returnvalue (Transformation|GetActorTransform))
  (bind _returnvalue_2 (Transformation|GetActorTransform))
  (bind _returnvalue_3 (Transformation|GetActorTransform))
  (bind _returnvalue_4 (Transformation|GetActorTransform))
  (bind (_location _rotation _scale) (Math|Transform|BreakTransform _returnvalue))
  (bind (_location_2 _rotation_2 _scale_2) (Math|Transform|BreakTransform _returnvalue_4))
  (bind (_location_3 _rotation_3 _scale_3) (Math|Transform|BreakTransform _returnvalue_2))
  (bind (_location_4 _rotation_4 _scale_4) (Math|Transform|BreakTransform _returnvalue_3))
  (bind _returnvalue_5 (* _scale 5e+01))
  (bind _returnvalue_6 (* _scale_4 5e+01))
  (bind _returnvalue_7 (* _scale_2 5e+01))
  (bind _returnvalue_8 (* _scale_3 5e+01))
  (switch int (Variables|Default|GetCutoffIndex)
    (:1
      (Rendering|Material|SetVectorParameterValue "/Game/Materials/MPC_CutoffArea.MPC_CutoffArea" "MinPoint_1" (Math|Conversions|ToLinearColor(Vector) (- _location_4 _returnvalue_6)) :!class /Script/Engine.KismetMaterialLibrary)
      (Rendering|Material|SetVectorParameterValue "/Game/Materials/MPC_CutoffArea.MPC_CutoffArea" "MaxPoint_1" (Math|Conversions|ToLinearColor(Vector) (+ _returnvalue_6 _location_4)) :!class /Script/Engine.KismetMaterialLibrary))
    (:2
      (Rendering|Material|SetVectorParameterValue "/Game/Materials/MPC_CutoffArea.MPC_CutoffArea" "MinPoint_2" (Math|Conversions|ToLinearColor(Vector) (- _location_2 _returnvalue_7)) :!class /Script/Engine.KismetMaterialLibrary)
      (Rendering|Material|SetVectorParameterValue "/Game/Materials/MPC_CutoffArea.MPC_CutoffArea" "MaxPoint_2" (Math|Conversions|ToLinearColor(Vector) (+ _returnvalue_7 _location_2)) :!class /Script/Engine.KismetMaterialLibrary))
    (:3
      (Rendering|Material|SetVectorParameterValue "/Game/Materials/MPC_CutoffArea.MPC_CutoffArea" "MinPoint_3" (Math|Conversions|ToLinearColor(Vector) (- _location_3 _returnvalue_8)) :!class /Script/Engine.KismetMaterialLibrary)
      (Rendering|Material|SetVectorParameterValue "/Game/Materials/MPC_CutoffArea.MPC_CutoffArea" "MaxPoint_3" (Math|Conversions|ToLinearColor(Vector) (+ _returnvalue_8 _location_3)) :!class /Script/Engine.KismetMaterialLibrary))
    (:4
      (Rendering|Material|SetVectorParameterValue "/Game/Materials/MPC_CutoffArea.MPC_CutoffArea" "MinPoint_4" (Math|Conversions|ToLinearColor(Vector) (- _location _returnvalue_5)) :!class /Script/Engine.KismetMaterialLibrary)
      (Rendering|Material|SetVectorParameterValue "/Game/Materials/MPC_CutoffArea.MPC_CutoffArea" "MaxPoint_4" (Math|Conversions|ToLinearColor(Vector) (+ _returnvalue_5 _location)) :!class /Script/Engine.KismetMaterialLibrary))))

(event EventBeginPlay
  (CallFunction|SetMaterialParameter))

(fn ConstructionScript
  (CallFunction|SetMaterialParameter))