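; Industrial robot arm that mounts a target tire at a destination point, presumably on a car.
; StartMountTire checks that the robot is idle and the tire is mountable, then plays the robot animation.
; Timed delays attach the tire to the arm's end socket, release it at the destination as "Mounted", then clear the busy flag.
; An older timeline-driven gripper pick-and-place path remains in the graph but is disconnected.
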(event Custom|StartMountTire
  (if (not (Variables|Default|GetIsBusy))
    (Utilities|IsValid (Variables|Default|GetTargetTire)
      (:Is%20Valid
        (if (Variables|/Game/Blueprints/BP_Tire.BP_Tire_C|GetCanBeMounted (Variables|Default|GetTargetTire))
          (Variables|Default|SetIsBusy true)
          (Variables|/Game/Blueprints/BP_Tire.BP_Tire_C|SetCanBeMounted (Variables|Default|GetTargetTire) false)
          (Components|Animation|PlayAnimation (Variables|Default|GetRobot) "/Game/Meshes/RobotLarge/SK_IndustrialRobot_Right_Anim.SK_IndustrialRobot_Right_Anim" false)
          (Utilities|FlowControl|Delay (Variables|Default|GetAttachTime))
          (Transformation|AttachComponentToComponent (Variables|Default|GetTargetTire) (Variables|Default|GetRobot) "Robot1_End" "SnapToTarget" "SnapToTarget" "KeepWorld" true)
          (Utilities|FlowControl|Delay (+ (Variables|Default|GetMountDuration) (- (Variables|Default|GetDetachTime) (Variables|Default|GetAttachTime))))
          (Transformation|DetachFromActor (Variables|Default|GetTargetTire) "KeepWorld" "KeepWorld" "KeepWorld")
          (Transformation|SetActorLocation (Variables|Default|GetTargetTire) (Transformation|GetWorldLocation (Variables|Default|GetDestPointRef)) false false)
          (Variables|/Game/Blueprints/BP_Tire.BP_Tire_C|SetCanBeMounted (Variables|Default|GetTargetTire) false)
          (Variables|/Game/Blueprints/BP_Tire.BP_Tire_C|SetTireState (Variables|Default|GetTargetTire) "Mounted")
          (Utilities|FlowControl|Delay (- (Variables|Default|GetAnimEndTime) (Variables|Default|GetDetachTime)))
          (Variables|Default|SetIsBusy false))))))

(fn ConstructionScript)