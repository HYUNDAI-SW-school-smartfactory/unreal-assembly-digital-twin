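; Procedural factory building generator that assembles a modular hall from instanced meshes on an XCount by YCount grid.
; GenerateFactory clears all instances, then loops over cells, deriving grid coordinates from the index to place floor, roof and roof-window tiles at fixed spacing.
; Walls appear only on perimeter cells, rotated to their edge, with corners getting two.
; A second loop places height-scaled pillars at every cell corner using a half-cell offset.
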(event Custom|GenerateFactory
  (Components|InstancedStaticMesh|ClearInstances (Variables|Default|GetFloorMesh))
  (for _index (range 0 (- (* (Variables|Default|GetXCount) (Variables|Default|GetYCount)) 1))
    (CallFunction|GenerateFloorandRoof _index)
    (CallFunction|GenerateWalls _index))
  (for _index_2 (range 0 (- (* (+ (Variables|Default|GetXCount) 1) (+ (Variables|Default|GetYCount) 1)) 1))
    (CallFunction|GeneratePillar _index_2)))

(fn ConstructionScript)

(fn GenerateFloorandRoof
  (params (Index :type Integer))
  (bind _xcount (Variables|Default|GetXCount))
  (bind _returnvalue (Math|Integer|%(Integer) Index _xcount))
  (bind _returnvalue_2 (/ Index _xcount))
  (bind _returnvalue_3 (Math|Conversions|ToFloat(Integer) _returnvalue_2))
  (bind _returnvalue_4 (Math|Conversions|ToFloat(Integer) _returnvalue))
  (bind _returnvalue_5 (Math|Vector|MakeVector _returnvalue_4 _returnvalue_3 0.0))
  (bind _returnvalue_6 (* _returnvalue_5 1.6e+03))
  (bind _returnvalue_7 (Math|Transform|MakeTransform _returnvalue_6))
  (Components|InstancedStaticMesh|AddInstance (Variables|Default|GetFloorMesh) _returnvalue_7 false)
  (Components|InstancedStaticMesh|AddInstance (Variables|Default|GetRoofMesh) _returnvalue_7 false)
  (Components|InstancedStaticMesh|AddInstance (Variables|Default|GetRoofWindowMesh) (Math|Transform|MakeTransform (+ _returnvalue_6 "0.000000,0.000000,-50.000000")) false))

(fn GenerateWalls
  (params (Index :type Integer))
  (bind _xcount (Variables|Default|GetXCount))
  (bind _xcount_2 (Variables|Default|GetXCount))
  (bind _xcount_3 (Variables|Default|GetXCount))
  (bind _returnvalue (Math|Integer|%(Integer) Index _xcount_2))
  (bind _returnvalue_2 (/ Index _xcount))
  (LocalVariables|SetFloorAndRoofLocation (* (Math|Vector|MakeVector (Math|Conversions|ToFloat(Integer) (Math|Integer|%(Integer) Index _xcount_3)) (Math|Conversions|ToFloat(Integer) (/ Index _xcount_3)) 0.0) 1.6e+03))
  (if (not (Math|Integer|InRange(Integer) _returnvalue 0 (- _xcount_2 1) false false))
    (Components|InstancedStaticMesh|AddInstance (Variables|Default|GetWallMesh) (Math|Transform|MakeTransform (LocalVariables|GetFloorAndRoofLocation) (Math|Rotator|SelectRotator "0.000000,-90.000000,0.000000" "0.000000,90.000000,0.000000" (== _returnvalue 0))) false))
  (if (not (Math|Integer|InRange(Integer) _returnvalue_2 0 (- (Variables|Default|GetYCount) 1) false false))
    (Components|InstancedStaticMesh|AddInstance (Variables|Default|GetWallMesh) (Math|Transform|MakeTransform (LocalVariables|GetFloorAndRoofLocation) (Math|Rotator|SelectRotator "0, 0, 0" "0.000000,180.000000,0.000000" (== _returnvalue_2 0))) false)))

(fn GeneratePillar
  (params (Index :type Integer))
  (bind _xcount (Variables|Default|GetXCount))
  (bind _returnvalue (+ _xcount 1))
  (Components|InstancedStaticMesh|AddInstance (Variables|Default|GetPillarMesh) (Math|Transform|MakeTransform (* (+ (Math|Vector|MakeVector (Math|Conversions|ToFloat(Integer) (Math|Integer|%(Integer) Index _returnvalue)) (Math|Conversions|ToFloat(Integer) (/ Index _returnvalue)) 0.0) "-0.500000,-0.500000,0.000000") 1.6e+03) "0, 0, 0" "1.000000,1.000000,1.350000") false))